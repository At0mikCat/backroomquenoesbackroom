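; BP_Corotrigger is a reusable trigger volume that fires a CoroTrigger event dispatcher when an actor with a configured tag overlaps it.
; Overlaps count only while Active, and an optional DoOnce gate limits firing to once until reset.
; ActivateTrigger re-arms that gate and enables the trigger, while DeactivateTrigger disables it.
; The construction script applies the configured box extent and 3D text label.
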(event Custom|ResetDoOnce
  (Utilities|FlowControl|DoOnce false) ; enters at Reset
)

(event Custom|ActivateTrigger
  (CallFunction|ResetDoOnce)
  (Variables|Default|SetActive? true))

(event Custom|DeactivateTrigger
  (Variables|Default|SetActive? false))

(event Collision|EventActorBeginOverlap
  (params (OtherActor :type Actor%20Object%20Reference))
  (if (Variables|Default|GetActive?)
    (if (Actor|ActorHasTag OtherActor (Variables|Default|GetTag))
      (if (Variables|Default|GetDoOnce)
        (Utilities|FlowControl|DoOnce false
          (:Completed
            _)))
      (Default|CallCoroTriggerDispatcher))))

(fn ConstructionScript
  (Components|Box|SetBoxExtent (Variables|Default|GetBox) (Variables|Default|GetSizeTrigger) true)
  (Variables|/Script/Text3D.Text3DComponent|SetText (Variables|Default|GetText3D) (Variables|Default|GetText)))