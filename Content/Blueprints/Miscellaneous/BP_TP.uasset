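; BP_TP is a teleporter trigger that moves the player to the location of a referenced TPLocation actor.
; When an actor tagged Player overlaps the Box, it shows a WD_Fade widget, plays a 2D sound, waits 1.5 seconds, then sets the actor's relative location to the target's world location.
; The construction script toggles the Niagara effect's visibility when the YesOrNo flag is set.
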(event OnComponentBeginOverlap(Box)
  (params (OverlappedComponent :type Primitive%20Component%20Object%20Reference) (OtherActor :type Actor%20Object%20Reference) (OtherComp :type Primitive%20Component%20Object%20Reference) (OtherBodyIndex :type Integer) (bFromSweep :type Boolean) (SweepResult :type Hit%20Result%20Structure%20%28by%20ref%29))
  (if (Actor|ActorHasTag OtherActor "Player")
    (bind _returnvalue (UserInterface|CreateWidget "/Game/UI/WD_Fade.WD_Fade_C"))
    (UserInterface|Viewport|AddtoViewport _returnvalue 0)
    (Audio|PlaySound2D (Variables|Default|GetSound) 1.0 1.0 0.0 0 0)
    (Utilities|FlowControl|Delay 1.5)
    (Transformation|SetActorRelativeLocation OtherActor (Transformation|GetWorldLocation (Variables|/Script/Engine.Actor|GetRootComponent (Variables|Default|GetTPLocation))))))

(fn ConstructionScript
  (if (Variables|Default|GetYesOrNo)
    (Rendering|ToggleVisibility (Variables|Default|GetNiagara) false)))