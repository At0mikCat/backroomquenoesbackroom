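; BP_Mimic is an enemy character that swaps Cube and Mimic visibility and activates when the player enters its alert trigger.
; Once active, Tick drives AI movement toward the player, followed by a delayed sphere-overlap attack with debug drawing, gated by CanAttack.
; Taking damage launches it along the axis to the damage causer, flags a movement-halting stagger and reduces health; Tick destroys it once dead.
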(event OnComponentBeginOverlap(TriggerAlert)
  (params (OverlappedComponent :type Primitive%20Component%20Object%20Reference) (OtherActor :type Actor%20Object%20Reference) (OtherComp :type Primitive%20Component%20Object%20Reference) (OtherBodyIndex :type Integer) (bFromSweep :type Boolean) (SweepResult :type Hit%20Result%20Structure%20%28by%20ref%29))
  ;[0.15 0.15 0.15 0.5] Alert
  (if (Actor|ActorHasTag OtherActor "Player")
    (Utilities|FlowControl|DoOnce false
      (:Completed
        (Rendering|ToggleVisibility (Variables|Default|GetCube) false)
        (Rendering|ToggleVisibility (Variables|Default|GetMimic) false)
        (Variables|Default|SetActivated true)))))

(event Custom|Movement
  (bind _collision (Variables|Default|GetCollision))
  (bind _attackrange (Variables|Default|GetAttackRange))
  (bind _returnvalue (Transformation|GetWorldLocation _collision))
  ;[0.15 0.15 0.15 0.5] Movement
  (if (Variables|Default|GetHitted?)
    (Components|Movement|StopMovementImmediately (Variables|Character|GetCharacterMovement))
    (Utilities|FlowControl|Delay 1.2)
    (Variables|Default|SetHitted? false)
    (Variables|Default|SetCanAttack true))
  (AI|AIMoveTo self "0, 0, 0" (Game|GetPlayerCharacter 0) 115.0 false
    (:OnSuccess
      (if (not (Variables|Default|GetCanAttack))
        (Utilities|FlowControl|Delay 0.2)
        (Variables|Default|SetCanAttack false)
        (Components|Movement|StopMovementImmediately (Variables|Character|GetCharacterMovement))
        (Utilities|FlowControl|Delay 1.2)
        (bind _outactors (Collision|SphereOverlapActors _returnvalue _attackrange (Utilities|Array|MakeArray "ObjectTypeQuery3") "/Game/FirstPersonTemplate/FirstPerson/Blueprints/BP_FirstPersonCharacter.BP_FirstPersonCharacter_C" (Utilities|Array|MakeArray self)))
        (Rendering|Debug|DrawDebugSphere _returnvalue _attackrange 12 "(R=1.000000,G=0.000000,B=0.185880,A=1.000000)" 2.0)
        (for _array_element _outactors
          (Game|Damage|ApplyDamage _array_element 4.0 (Pawn|GetController) self "/Script/Engine.DamageType")
          (Utilities|FlowControl|Delay 6.0)
          (Variables|Default|SetCanAttack true))))))

(event EventTick
  (params (DeltaSeconds :type Float%20%28single-precision%29))
  ;[0.15 0.15 0.15 0.5] Event Tick
  (Utilities|FlowControl|Sequence
    (:then_0
      (if (Variables|Default|GetActivated)
        (CallFunction|Movement)))
    (:then_1
      (if (Variables|Default|GetDead?)
        (Development|PrintString "Murio")
        (Actor|DestroyActor)))))

(event Game|Damage|EventAnyDamage
  (params (Damage :type Float%20%28single-precision%29) (DamageType :type Damage%20Type%20Object%20Reference) (InstigatedBy :type Controller%20Object%20Reference) (DamageCauser :type Actor%20Object%20Reference))
  ;[0.15 0.15 0.15 0.5] ReceiveDamage...and Knockback
  (bind _output_get (Variables|Default|SetDirection (Math|Vector|Normalize (- (Transformation|GetActorLocation DamageCauser) (Transformation|GetActorLocation)) 1.0)))
  (Variables|Default|SetHitted? true)
  (Character|LaunchCharacter (* _output_get (Variables|Default|GetForce)) false false)
  (if (not (Variables|Default|GetDead?))
    (Variables|Default|SetHPActual (- (Variables|Default|GetHPActual) Damage))
    (if (<= (Variables|Default|GetHPActual) 0.0)
      (Variables|Default|SetDead? true))))

(fn ConstructionScript)