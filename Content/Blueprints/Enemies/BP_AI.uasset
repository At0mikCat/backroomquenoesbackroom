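; BP_AI is an enemy character that makes melee attacks and reacts to damage.
; Attack plays a zombie montage, then after a delay sphere-traces forward for pawns to apply damage, re-arming when the montage ends.
; Damage flags Hitted on the BP_AIController blackboard, then lowers HP with a sound and hit-reaction montage.
; Tick sets Dead at a low HP threshold, so the next hit triggers ragdoll and delayed destruction.
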(event Game|Damage|EventAnyDamage
  (params (Damage :type Float%20%28single-precision%29) (DamageType :type Damage%20Type%20Object%20Reference) (InstigatedBy :type Controller%20Object%20Reference) (DamageCauser :type Actor%20Object%20Reference))
  (bind _asbp_aicontroller (Utilities|Casting|CastToBP_AIController (Pawn|GetController)))
  (AI|Components|Blackboard|SetValueasBool (AI|GetBlackboard _asbp_aicontroller) (Variables|Default|GetHitted) true)
  (if (Variables|Default|GetDead?)
    (Audio|PlaySoundatLocation "/Game/Sound/MimicDeath1.MimicDeath1" (Transformation|GetActorLocation) "0, 0, 0" 1.0 1.0 0.0 "/Game/Sound/NaturalAttenuation.NaturalAttenuation" 0 0 0)
    (Physics|SetSimulatePhysics (Variables|Character|GetMesh) true)
    (Utilities|FlowControl|Delay 2.0)
    (Actor|DestroyActor)
    (else
      (bind _output_get (Variables|Default|SetHP (- (Variables|Default|GetHP) Damage)))
      (Development|PrintString (Utilities|String|ToString(Float) _output_get))
      (Audio|PlaySoundatLocation "/Game/Sound/MimicDamage.MimicDamage" (Transformation|GetActorLocation) "0, 0, 0" 1.0 1.0 0.0 0 0 0 0)
      (Animation|Montage|PlayMontage (Variables|Character|GetMesh) "/Game/Imported/Assets/Enemy/Standing_React_Death_Backward_Montage.Standing_React_Death_Backward_Montage"))))

(event EventTick
  (params (DeltaSeconds :type Float%20%28single-precision%29))
  (if (<= (Variables|Default|GetHP) 4.0)
    (Variables|Default|SetDead? true)))

(event EventAttack
  (bind _returnvalue (Transformation|GetActorLocation))
  (if (Variables|Default|GetCanAttack)
    (Animation|Montage|PlayMontage (Variables|Character|GetMesh) "/Game/Imported/Assets/Enemy/Zombie_Attack_Montage.Zombie_Attack_Montage"
      (:then
        (Variables|Default|SetCanAttack false)
        (Utilities|FlowControl|Delay 1.0)
        (bind (_outhit _returnvalue_2) (Collision|SphereTraceForObjects _returnvalue (+ _returnvalue (* (Math|Vector|GetForwardVector (Transformation|GetActorRotation)) 1e+02)) 1e+02 (Utilities|Array|MakeArray "ObjectTypeQuery3") false 0 "None" true "(R=0.938138,G=0.000000,B=1.000000,A=1.000000)" "(R=0.000000,G=1.000000,B=0.000000,A=1.000000)" 0.5))
        (if _returnvalue_2
          (Game|Damage|ApplyDamage (.HitActor (Collision|BreakHitResult _outhit)) 4.0 0 0)))
      (:OnCompleted
        (Variables|Default|SetCanAttack true :!label _label))
      (:OnInterrupted
        (goto _label)))))

(fn ConstructionScript)