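; Enemy Blueprint for subject 03 that acts as an audio lure and a scripted voice encounter.
; A Delay on Tick spawns the Random sound at the actor every six seconds until InZone is set, keeping its audio component.
; When a Player-tagged actor enters the Box, it sets InZone, toggles that component, and plays two timed voice clips while player movement is disabled, then restores walking.
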(event OnComponentBeginOverlap(Box)
  (params (OverlappedComponent :type Primitive%20Component%20Object%20Reference) (OtherActor :type Actor%20Object%20Reference) (OtherComp :type Primitive%20Component%20Object%20Reference) (OtherBodyIndex :type Integer) (bFromSweep :type Boolean) (SweepResult :type Hit%20Result%20Structure%20%28by%20ref%29))
  (bind _returnvalue (Game|GetPlayerCharacter 0))
  (bind _asbp_first_person_character (Utilities|Casting|CastToBP_FirstPersonCharacter _returnvalue))
  (if (Actor|ActorHasTag OtherActor "Player")
    (Variables|Default|SetInZone? true)
    (Components|Activation|ToggleActive (Variables|Default|GetReturn))
    (Audio|SpawnSound2D "/Game/Imported/Musica/Sujeto03/Sujeto03Voz5.Sujeto03Voz5" 1.0 1.0 0.0 0)
    (Pawn|Components|CharacterMovement|DisableMovement (Variables|/Script/Engine.Character|GetCharacterMovement _asbp_first_person_character))
    (Utilities|FlowControl|Delay 3.0)
    (Audio|PlaySoundatLocation "/Game/Imported/Assets/Sonidos/PACIENTE08_-_PROTA/08Voz7.08Voz7" (Transformation|GetActorLocation (Game|GetPlayerCharacter 0)) "0, 0, 0" 0.6 1.0 0.0 0 0 0 0)
    (Utilities|FlowControl|Delay 3.0)
    (Pawn|Components|CharacterMovement|SetMovementMode (Variables|/Script/Engine.Character|GetCharacterMovement _asbp_first_person_character) "MOVE_Walking" 0)))

(event Collision|EventActorBeginOverlap
  (params (OtherActor :type Actor%20Object%20Reference)))

(event EventTick
  (params (DeltaSeconds :type Float%20%28single-precision%29))
  (Utilities|FlowControl|Delay 6.0)
  (if (not (Variables|Default|GetInZone?))
    (bind _returnvalue (Audio|SpawnSoundatLocation "/Game/Sound/Random.Random" (Transformation|GetActorLocation) "0, 0, 0" 1.0 1.0 0.0 "/Game/Sound/NaturalAttenuation.NaturalAttenuation" 0))
    (Variables|Default|SetReturn _returnvalue)))

(fn ConstructionScript)