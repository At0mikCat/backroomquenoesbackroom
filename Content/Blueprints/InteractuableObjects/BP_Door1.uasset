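; BP_Door1 is an interactable door that toggles between open and closed on each Interact event.
; Interact fires an activated dispatcher, then a FlipFlop alternates between playing and reversing a Timeline that lerps the Scene component's relative rotation, with a 2D sound only on the forward swing.
; The construction script copies ChildConfig's prompt text, trigger radius, do-once and active settings into its BP_InteractChild child actor.
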(event EventInteract
  (Default|CallActivatedDispatcher)
  (Utilities|FlowControl|FlipFlop
    (:A
      (Audio|PlaySound2D (Variables|Default|GetSound) 1.0 1.0 0.0 0 0)
      (bind _doorfloat (Timeline|Timeline Play)
        (:Update
          (Transformation|SetRelativeRotation (Variables|Default|GetScene) (Math|Rotator|Lerp(Rotator) "0, 0, 0" "0.000000,-180.000000,0.000000" _doorfloat) false false))))
    (:B
      (Timeline|Timeline Reverse))))

(fn ConstructionScript
  (bind _childconfig (Variables|Default|GetChildConfig))
  (bind (_objectname _objectradius _doonce _active_) (Utilities|Struct|BreakBS_InteractionChildStructure _childconfig))
  (bind _asbp_interact_child (Utilities|Casting|CastToBP_InteractChild (Variables|/Script/Engine.ChildActorComponent|GetChildActor (Variables|Default|GetChildActor))))
  (Variables|/Game/Blueprints/InteractuableObjects/BP_InteractChild.BP_InteractChild_C|SetInteractText _asbp_interact_child _objectname)
  (Components|Sphere|SetSphereRadius (Variables|/Game/Blueprints/InteractuableObjects/BP_InteractChild.BP_InteractChild_C|GetSphere _asbp_interact_child) _objectradius true)
  (Variables|/Game/Blueprints/InteractuableObjects/BP_InteractChild.BP_InteractChild_C|SetDoOnce _asbp_interact_child _doonce)
  (Variables|/Game/Blueprints/InteractuableObjects/BP_InteractChild.BP_InteractChild_C|SetActive? _asbp_interact_child _active_))