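; BP_InteractChild is an interaction point used as a child actor, relaying interaction to its parent actor.
; ActiveChild calls InteractMessage on the parent, either through a one-shot gate that also disables the collision sphere, or whenever Active when DoOnce is off.
; EnableInteract and DisableInteract toggle Active and the sphere's collision, with enabling also re-arming the gate.
; The sphere starts without collision when inactive.
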(event Custom|ResetDoOnce
  (Utilities|FlowControl|DoOnce false) ; enters at Reset
)

(event EventBeginPlay
  (if (not (Variables|Default|GetActive?))
    (Collision|SetCollisionEnabled (Variables|Default|GetSphere) "NoCollision")))

(event EventActiveChild
  (bind _returnvalue (Actor|GetParentActor))
  (Utilities|IsValid _returnvalue
    (:Is%20Valid
      (if (Variables|Default|GetDoOnce)
        (Utilities|FlowControl|DoOnce false
          (:Completed
            (Class|InteractInterface|Interact(Message) _returnvalue)
            (Collision|SetCollisionEnabled (Variables|Default|GetSphere) "NoCollision")))
        (elif (Variables|Default|GetActive?)
          (Class|InteractInterface|Interact(Message) _returnvalue))))))

(event EventEnableInteract
  (CallFunction|ResetDoOnce)
  (Variables|Default|SetActive? true)
  (Collision|SetCollisionEnabled (Variables|Default|GetSphere) "QueryAndPhysics"))

(event EventDisableInteract
  (Variables|Default|SetActive? false)
  (Collision|SetCollisionEnabled (Variables|Default|GetSphere) "NoCollision"))

(fn ConstructionScript)