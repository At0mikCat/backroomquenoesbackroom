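; BP_Note is an interactable note that opens and closes a full-screen Notes widget on alternate interactions.
; Interact fires the activated dispatcher, then a FlipFlop either shows the widget with sounds and locks look and move input, or removes it, restores input and toggles the spawned sound.
; The construction script copies ChildConfig's name, radius, DoOnce and Active settings into its BP_InteractChild child actor.
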(event EventInteract
  (bind _returnvalue (Game|GetPlayerController 0))
  (Default|CallActivatedDispatcher)
  (Utilities|FlowControl|FlipFlop
    (:A
      (Audio|PlaySound2D (Variables|Default|GetSound_0) 1.0 1.0 0.0 0 0)
      (bind _returnvalue_2 (UserInterface|CreateWidget (Variables|Default|GetNotes)))
      (bind _output_get (Variables|Default|SetNote _returnvalue_2))
      (UserInterface|Viewport|AddtoViewport _output_get 1)
      (Input|SetIgnoreLookInput _returnvalue true)
      (Input|SetIgnoreMoveInput _returnvalue true)
      (bind _returnvalue_3 (Audio|SpawnSound2D (Variables|Default|GetSound) 1.0 1.0 0.0 0))
      (Variables|Default|SetSoundVar _returnvalue_3))
    (:B
      (Widget|RemovefromParent (Variables|Default|GetNote))
      (Input|SetIgnoreLookInput _returnvalue false)
      (Input|SetIgnoreMoveInput _returnvalue false)
      (Components|Activation|ToggleActive (Variables|Default|GetSoundVar)))))

(fn ConstructionScript
  (bind _childconfig (Variables|Default|GetChildConfig))
  (bind (_objectname _objectradius _doonce _active_) (Utilities|Struct|BreakBS_InteractionChildStructure _childconfig))
  (bind _asbp_interact_child (Utilities|Casting|CastToBP_InteractChild (Variables|/Script/Engine.ChildActorComponent|GetChildActor (Variables|Default|GetChildActor))))
  (Variables|/Game/Blueprints/InteractuableObjects/BP_InteractChild.BP_InteractChild_C|SetInteractText _asbp_interact_child _objectname)
  (Components|Sphere|SetSphereRadius (Variables|/Game/Blueprints/InteractuableObjects/BP_InteractChild.BP_InteractChild_C|GetSphere _asbp_interact_child) _objectradius true)
  (Variables|/Game/Blueprints/InteractuableObjects/BP_InteractChild.BP_InteractChild_C|SetDoOnce _asbp_interact_child _doonce)
  (Variables|/Game/Blueprints/InteractuableObjects/BP_InteractChild.BP_InteractChild_C|SetActive? _asbp_interact_child _active_))