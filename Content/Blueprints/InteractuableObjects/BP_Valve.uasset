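; BP_Valve is an interactable valve that spins when used and adds to a valve count kept in BP_GameInstance.
; Interact fires an Activated dispatcher, increments and prints that counter, plays a 2D sound, then drives a full yaw turn of the Scene component through a Timeline.
; The construction script pushes ChildConfig settings (prompt text, radius, DoOnce, Active) into its BP_InteractChild child actor.
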(event EventInteract
  (Default|CallActivatedDispatcher)
  (bind _asbp_game_instance (Utilities|Casting|CastToBP_GameInstance (Game|GetGameInstance)))
  (bind _output_get (Variables|/Game/Blueprints/InteractuableObjects/BP_GameInstance.BP_GameInstance_C|SetValveCounter _asbp_game_instance (+ (Variables|/Game/Blueprints/InteractuableObjects/BP_GameInstance.BP_GameInstance_C|GetValveCounter _asbp_game_instance) 1)))
  (Development|PrintString (Utilities|String|ToString(Integer) _output_get))
  (Audio|PlaySound2D (Variables|Default|GetSound) 1.0 1.0 0.0 0 0)
  (bind _doorfloat (Timeline|Timeline Play)
    (:Update
      (Transformation|SetRelativeRotation (Variables|Default|GetScene) (Math|Rotator|Lerp(Rotator) "0, 0, 0" "-360.000000,0.000000,0.000000" _doorfloat) false false))))

(fn ConstructionScript
  (bind _childconfig (Variables|Default|GetChildConfig))
  (bind (_objectname _objectradius _doonce _active_) (Utilities|Struct|BreakBS_InteractionChildStructure _childconfig))
  (bind _asbp_interact_child (Utilities|Casting|CastToBP_InteractChild (Variables|/Script/Engine.ChildActorComponent|GetChildActor (Variables|Default|GetChildActor))))
  (Variables|/Game/Blueprints/InteractuableObjects/BP_InteractChild.BP_InteractChild_C|SetInteractText _asbp_interact_child _objectname)
  (Components|Sphere|SetSphereRadius (Variables|/Game/Blueprints/InteractuableObjects/BP_InteractChild.BP_InteractChild_C|GetSphere _asbp_interact_child) _objectradius true)
  (Variables|/Game/Blueprints/InteractuableObjects/BP_InteractChild.BP_InteractChild_C|SetDoOnce _asbp_interact_child _doonce)
  (Variables|/Game/Blueprints/InteractuableObjects/BP_InteractChild.BP_InteractChild_C|SetActive? _asbp_interact_child _active_))